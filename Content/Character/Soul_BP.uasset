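; Player character Soul, which cycles through owned elemental forms, each changing its materials, particles, light color and voice.
; Fire shoots projectiles aimed by camera trace, Air enables jumping, and Water moves faster inside speed-up volumes.
; Switches notify SoulGameState, and elemental ones trigger overlapping teleportation puzzles.
; It also handles camera-relative movement with sound and dust, JumpBox jump boosts, and a single orbiting catalyst that can be spent.
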(event Custom|Fire
  (bind _soulparticles (Variables|Components|GetSoulParticles))
  (bind _camera (Variables|Components|GetCamera))
  (bind _returnvalue (Transformation|GetWorldLocation _soulparticles))
  (bind _returnvalue_2 (Transformation|GetWorldLocation _camera))
  ;[1 1 1] Shooting
  (Utilities|FlowControl|Sequence
    (:then_0
      (Utilities|FlowControl|DoOnce false :!label _label
        (:Completed
          (bind (_outhit _returnvalue_3) (Collision|LineTraceByChannel _returnvalue_2 (+ _returnvalue_2 (* (Math|Vector|GetForwardVector _camera) 1e+05)) "TraceTypeQuery1" false 0 "None"))
          (bind _returnvalue_4 (Game|SpawnActorfromClass "/Game/Character/Projectile/BP_Projectile.BP_Projectile_C" (Math|Transform|MakeTransform _returnvalue (Math|Rotator|MakeRotator (.roll (Math|Rotator|FindLookatRotation _returnvalue (Math|Vector|SelectVector (.ImpactPoint (Collision|BreakHitResult _outhit)) (.TraceEnd (Collision|BreakHitResult _outhit)) _returnvalue_3))) (.pitch (Math|Rotator|FindLookatRotation _returnvalue (Math|Vector|SelectVector (.ImpactPoint (Collision|BreakHitResult _outhit)) (.TraceEnd (Collision|BreakHitResult _outhit)) _returnvalue_3))) (.yaw (Math|Rotator|FindLookatRotation _returnvalue (Math|Vector|SelectVector (.ImpactPoint (Collision|BreakHitResult _outhit)) (.TraceEnd (Collision|BreakHitResult _outhit)) _returnvalue_3))))) "Undefined" 0 0))
          (Class|Actor|AddActorLocalTransform _returnvalue_4 (Math|Transform|MakeTransform "100.000000,0.000000,0.000000" "0.000000,90.000000, 0" "0.300000,0.300000,0.300000") false false)
          (Audio|Components|Audio|Play (Variables|Default|GetSFX_FireIn) 0.0))))
    (:then_1
      (Utilities|FlowControl|Delay 0.3)
      (goto _label Reset))))

(event Custom|AddOrbitingCatalyst
  ;[1 1 1] Handling Orbiting Catalysts
  (Utilities|FlowControl|DoOnce false
    (:Completed
      (bind _returnvalue (AddComponent|AddChildActorComponent false (Math|Transform|MakeTransform "0,100.000000, 0" "0, 0, 0" "1,1,1")))
      (ChildActorComponent|SetChildActorClass _returnvalue "/Game/Blueprints/Level_Objs/Catalyst/BP_OrbitingCatalyst.BP_OrbitingCatalyst_C")
      (Variables|Default|SetOrbitingCatalystRef _returnvalue)
      (Audio|Components|Audio|Play (Variables|Default|GetSFX_CatalystGet) 0.0)
      (Utilities|FlowControl|DoOnce false) ; enters at Reset
    )))

(event Custom|WasteCatalyst
  ;[1 1 1] Handling Orbiting Catalysts
  (Utilities|FlowControl|DoOnce false
    (:Completed
      (Components|DestroyComponent (Variables|Default|GetOrbitingCatalystRef))
      (Utilities|FlowControl|DoOnce false) ; enters at Reset
    )))

(event EventBeginPlay
  (bind _ascharacter_movement_component (Utilities|Casting|CastToCharacterMovementComponent (Pawn|GetMovementComponent)))
  (Variables|Default|SetMovementComponent _ascharacter_movement_component)
  (CallFunction|TransformDefault)
  (bind _assoul_game_state_base (Utilities|Casting|CastToSoulGameStateBase (Game|GetGameState)))
  (Variables|Default|SetSoulGameStateRef _assoul_game_state_base))

(event EventTick
  (params (DeltaSeconds :type Float%20%28single-precision%29))
  (Utilities|FlowControl|Sequence
    (:then_0
      ;[1 1 1] Water Speed Up
      (if (Utilities|Enum|Equal(Enum) (Variables|Default|GetElementalState) "NewEnumerator2")
        (Variables|/Script/Engine.CharacterMovementComponent|SetMaxWalkSpeed (Variables|Default|GetMovementComponent) 6e+02)
        (if (Utilities|Array|IsValidIndex (Collision|GetOverlappingActors (Variables|Collision|GetCapsuleComponent) "/Game/Blueprints/Level_Objs/WaterSpeedUpVolume.WaterSpeedUpVolume_C" :!class /Script/Engine.PrimitiveComponent))
          (Variables|/Script/Engine.CharacterMovementComponent|SetMaxWalkSpeed (Variables|Default|GetMovementComponent) 1.2e+03))))
    (:then_1
      ;[1 1 1] Sky Stone Jump
      (for _array_element (Class|PrimitiveComponent|GetOverlappingComponents (Variables|Collision|GetCapsuleComponent))
        (bind _asmoveable_object_with_reverse (Utilities|Casting|CastToMoveableObject_with_reverse (Utilities|Array|Get(acopy) (Collision|GetOverlappingActors (Variables|Collision|GetCapsuleComponent) "/Game/Blueprints/Level_Objs/MoveableObject_with_reverse.MoveableObject_with_reverse_C" :!class /Script/Engine.PrimitiveComponent))))
        (if (== _array_element (Variables|/Game/Blueprints/Level_Objs/MoveableObject_with_reverse.MoveableObject_with_reverse_C|GetJumpBox _asmoveable_object_with_reverse))
          (Variables|/Script/Engine.CharacterMovementComponent|SetJumpZVelocity (Variables|Default|GetMovementComponent) 9e+02)
          (else
            (Variables|/Script/Engine.CharacterMovementComponent|SetJumpZVelocity (Variables|Default|GetMovementComponent) 6e+02)))))))

(event Input|ActionEvents|InputActionJump
  (params (Key :type Key%20Structure :default "None"))
  ;[1 1 1] Basic Moveent and Camera Setup
  (:Pressed
    (if (Utilities|Enum|Equal(Enum) (Variables|Default|GetElementalState) "NewEnumerator3")
      (Character|Jump))))

(event Input|ActionEvents|InputActionFire
  (params (Key :type Key%20Structure :default "None"))
  ;[1 1 1] Shooting
  (:Pressed
    (if (Utilities|Enum|Equal(Enum) (Variables|Default|GetElementalState) "NewEnumerator1")
      (CallFunction|Fire))))

(event Input|ActionEvents|InputActionNextElementalAbility
  (params (Key :type Key%20Structure :default "None"))
  ;[1 1 1] Changing Abilities Action Inputs
  (:Pressed
    (CallFunction|SetNextElementalAbility)))

(event Input|ActionEvents|InputActionPreviousElementalAbility
  (params (Key :type Key%20Structure :default "None"))
  ;[1 1 1] Changing Abilities Action Inputs
  (:Pressed
    (CallFunction|SetPreviousElementalAbility)))

(event Input|AxisEvents|InputAxisForward
  (params (AxisValue :type Float%20%28single-precision%29))
  ;[1 1 1] Basic Moveent and Camera Setup
  (Pawn|Input|AddMovementInput (Math|Vector|GetForwardVector (Math|Rotator|MakeRotator 0.0 0.0 (.Yaw (Math|Rotator|BreakRotator (Pawn|GetControlRotation :!class /Script/Engine.Pawn))))) AxisValue false)
  (Utilities|PlayMovementSound AxisValue (stale Input|AxisEvents|InputAxisRight AxisValue)
    (:Out
      (Utilities|SetParticleEmission AxisValue (stale Input|AxisEvents|InputAxisRight AxisValue)))))

(event Input|AxisEvents|InputAxisRight
  (params (AxisValue :type Float%20%28single-precision%29))
  ;[1 1 1] Basic Moveent and Camera Setup
  (Pawn|Input|AddMovementInput (Math|Vector|GetRightVector (Math|Rotator|MakeRotator 0.0 0.0 (.Yaw (Math|Rotator|BreakRotator (Pawn|GetControlRotation :!class /Script/Engine.Pawn))))) AxisValue false))

(event Input|AxisEvents|InputAxisLookUp
  (params (AxisValue :type Float%20%28single-precision%29))
  ;[1 1 1] Basic Moveent and Camera Setup
  (Pawn|Input|AddControllerPitchInput AxisValue))

(event Input|AxisEvents|InputAxisLookRight
  (params (AxisValue :type Float%20%28single-precision%29))
  ;[1 1 1] Basic Moveent and Camera Setup
  (Pawn|Input|AddControllerYawInput AxisValue))

(fn ConstructionScript)

(fn TransformDefault
  (bind _soulparticles (Variables|Components|GetSoulParticles))
  (Variables|Default|SetElementalState "NewEnumerator0")
  (Rendering|SetVisibility (Variables|Default|Getaura) false false)
  (Rendering|Material|SetMaterial (Variables|Default|GetBody) 0 "/Game/Character/MagicBallMaterial/BodyNeutral_Inst.BodyNeutral_Inst")
  (Rendering|SetVisibility (Variables|Default|Getshell) false false)
  (Effects|Components|ParticleSystem|SetTemplate _soulparticles "/Game/Character/P_Soul_particle.P_Soul_particle")
  (Rendering|SetVisibility _soulparticles false false))

(fn TrasformWater
  (bind _shell (Variables|Default|Getshell))
  (bind _body (Variables|Default|GetBody))
  (Variables|Default|SetElementalState "NewEnumerator2")
  (Rendering|SetVisibility _body true false)
  (Rendering|Material|SetMaterial _body 0 "/Game/Character/MagicBallMaterial/BodyWater_Inst.BodyWater_Inst")
  (Rendering|SetVisibility _shell true false)
  (Rendering|Material|SetMaterial _shell 0 "/Game/WaterMaterials/Materials/M_Lake.M_Lake")
  (Rendering|SetVisibility (Variables|Components|GetSoulParticles) false false)
  (Effects|Components|ParticleSystem|SetIntParameter (Variables|Default|GetElementVoice_SoundCue) "Index" 3)
  (Audio|Components|Audio|Play (Variables|Default|GetElementVoice_SoundCue) 0.0)
  (Rendering|Components|Light|SetLightColor (Variables|Default|GetSoulLight) "(R=0.108272,G=0.097794,B=0.894118,A=1.000000)" true))

(fn TransformAir
  (bind _shell (Variables|Default|Getshell))
  (bind _body (Variables|Default|GetBody))
  (Variables|Default|SetElementalState "NewEnumerator3")
  (Rendering|SetVisibility _body true false)
  (Rendering|Material|SetMaterial _body 0 "/Game/Character/MagicBallMaterial/BodyAir_Inst.BodyAir_Inst")
  (Rendering|SetVisibility _shell true false)
  (Rendering|Material|SetMaterial _shell 0 "/Game/WaterMaterials/Materials/M_Waterfall.M_Waterfall")
  (Rendering|SetVisibility (Variables|Components|GetSoulParticles) false false)
  (Effects|Components|ParticleSystem|SetIntParameter (Variables|Default|GetElementVoice_SoundCue) "Index" 0)
  (Audio|Components|Audio|Play (Variables|Default|GetElementVoice_SoundCue) 0.0)
  (Rendering|Components|Light|SetLightColor (Variables|Default|GetSoulLight) "(R=0.243137,G=0.490196,B=0.450980,A=0.000000)" true))

(fn TransformFire
  (bind _soulparticles (Variables|Components|GetSoulParticles))
  (bind _body (Variables|Default|GetBody))
  (Variables|Default|SetElementalState "NewEnumerator1")
  (Rendering|SetVisibility _body true false)
  (Rendering|Material|SetMaterial _body 0 "/Game/Character/MagicBallMaterial/BodyFire_Inst.BodyFire_Inst")
  (Rendering|SetVisibility (Variables|Default|Getshell) false false)
  (Effects|Components|ParticleSystem|SetTemplate _soulparticles "/Game/Character/P_Fire.P_Fire")
  (Rendering|SetVisibility _soulparticles true false)
  (Effects|Components|ParticleSystem|SetIntParameter (Variables|Default|GetElementVoice_SoundCue) "Index" 2)
  (Audio|Components|Audio|Play (Variables|Default|GetElementVoice_SoundCue) 0.0)
  (Rendering|Components|Light|SetLightColor (Variables|Default|GetSoulLight) "(R=0.490196,G=0.003922,B=0.000000,A=0.000000)" true))

(fn SetNextElementalAbility
  (bind _ownedelements (Variables|Default|GetOwnedElements))
  (if (> (Utilities|Set|Length _ownedelements) 1)
    (bind _result (Utilities|Set|ToArray _ownedelements))
    (if (== (Utilities|Array|FindItem _result (Variables|Default|GetElementalState)) (- (Utilities|Array|Length _result) 1))
      (bind _output_get (LocalVariables|SetNextElementIndex 0))
      (else
        (bind _output_get_2 (LocalVariables|SetNextElementIndex (+ (Utilities|Array|FindItem _result (Variables|Default|GetElementalState)) 1)))))
    (CallFunction|ChangeStatebyIndex _output_get)))

(fn SetPreviousElementalAbility
  (bind _ownedelements (Variables|Default|GetOwnedElements))
  (if (> (Utilities|Set|Length _ownedelements) 1)
    (bind _result (Utilities|Set|ToArray _ownedelements))
    (if (== (Utilities|Array|FindItem _result (Variables|Default|GetElementalState)) 0)
      (bind _output_get (LocalVariables|SetNextElementIndex (- (Utilities|Array|Length _result) 1)))
      (CallFunction|ChangeStatebyIndex _output_get)
      (else
        (bind _output_get_2 (LocalVariables|SetNextElementIndex (- (Utilities|Array|FindItem _result (Variables|Default|GetElementalState)) 1)))
        (CallFunction|ChangeStatebyIndex _output_get_2)))))

(fn ChangeStatebyIndex
  (params (index :type Integer))
  (bind _result (Utilities|Set|ToArray (Variables|Default|GetOwnedElements)))
  (bind _output_get (Variables|Default|SetElementalState (Utilities|Array|Get(acopy) _result index)))
  (Default|NoifyStateChange (Variables|Default|GetSoulGameStateRef) _output_get)
  (switch Utilities|FlowControl|Switch|SwitchonSoulElementalState _output_get
    (:NewEnumerator0
      (CallFunction|TransformDefault))
    (:NewEnumerator1
      (CallFunction|TransformFire)
      (for _array_element (Class|PrimitiveComponent|GetOverlappingComponents (Variables|Collision|GetCapsuleComponent)) :!label _label
        (bind _asteleportation_puzzle (Utilities|Casting|CastToTeleportationPuzzle (Utilities|Array|Get(acopy) (Collision|GetOverlappingActors (Variables|Collision|GetCapsuleComponent) "/Game/Blueprints/Level_Objs/TeleportationPuzzle.TeleportationPuzzle_C" :!class /Script/Engine.PrimitiveComponent))))
        (if (== _array_element (Variables|/Game/Blueprints/Level_Objs/TeleportationPuzzle.TeleportationPuzzle_C|GetTeleportationVolume _asteleportation_puzzle))
          (Default|TeleportationAttempt _asteleportation_puzzle))))
    (:NewEnumerator2
      (CallFunction|TrasformWater)
      (goto _label))
    (:NewEnumerator3
      (CallFunction|TransformAir)
      (goto _label))))