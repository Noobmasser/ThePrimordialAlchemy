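; Teleportation puzzle level object that sends the Soul_BP back to a stored location when it enters the teleportation volume, unless it is in one particular elemental state.
; The destination starts at a default target point, and each of five trigger volumes switches it to its matching target point when the Soul_BP overlaps it.
; A teleport plays a 2D sound and passes the soul's own rotation along with the stored destination.
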(event OnComponentBeginOverlap(TeleportationVolume)
  (params (OverlappedComponent :type Primitive%20Component%20Object%20Reference) (OtherActor :type Actor%20Object%20Reference) (OtherComp :type Primitive%20Component%20Object%20Reference) (OtherBodyIndex :type Integer) (bFromSweep :type Boolean) (SweepResult :type Hit%20Result%20Structure%20%28by%20ref%29))
  (bind (_teleportationlocation_x _teleportationlocation_y _teleportationlocation_z) (|getTeleportationXY))
  (bind _assoul_bp (Utilities|Casting|CastToSoul_BP OtherActor))
  (if (not (Utilities|Enum|Equal(Enum) (Variables|/Game/Character/Soul_BP.Soul_BP_C|GetElementalState _assoul_bp) "NewEnumerator1"))
    (Audio|PlaySound2D (Variables|Default|GetSound) 1.0 1.0 0.0 0 0)
    (Transformation|Teleport _assoul_bp (Math|Vector|MakeVector _teleportationlocation_x _teleportationlocation_y _teleportationlocation_z) (|getRotation _assoul_bp))))

(event OnComponentBeginOverlap(TriggerVolume1)
  (params (OverlappedComponent :type Primitive%20Component%20Object%20Reference) (OtherActor :type Actor%20Object%20Reference) (OtherComp :type Primitive%20Component%20Object%20Reference) (OtherBodyIndex :type Integer) (bFromSweep :type Boolean) (SweepResult :type Hit%20Result%20Structure%20%28by%20ref%29))
  (Utilities|Casting|CastToSoul_BP OtherActor)
  (Variables|Default|SetTeleportationLocation (Transformation|GetWorldLocation (Variables|Default|GetTargetPoint1))))

(event OnComponentBeginOverlap(TriggerVolume2)
  (params (OverlappedComponent :type Primitive%20Component%20Object%20Reference) (OtherActor :type Actor%20Object%20Reference) (OtherComp :type Primitive%20Component%20Object%20Reference) (OtherBodyIndex :type Integer) (bFromSweep :type Boolean) (SweepResult :type Hit%20Result%20Structure%20%28by%20ref%29))
  (Utilities|Casting|CastToSoul_BP OtherActor)
  (Variables|Default|SetTeleportationLocation (Transformation|GetWorldLocation (Variables|Default|GetTargetPoint2))))

(event OnComponentBeginOverlap(TriggerVolume3)
  (params (OverlappedComponent :type Primitive%20Component%20Object%20Reference) (OtherActor :type Actor%20Object%20Reference) (OtherComp :type Primitive%20Component%20Object%20Reference) (OtherBodyIndex :type Integer) (bFromSweep :type Boolean) (SweepResult :type Hit%20Result%20Structure%20%28by%20ref%29))
  (Utilities|Casting|CastToSoul_BP OtherActor)
  (Variables|Default|SetTeleportationLocation (Transformation|GetWorldLocation (Variables|Default|GetTargetPoint3))))

(event OnComponentBeginOverlap(TriggerVolume4)
  (params (OverlappedComponent :type Primitive%20Component%20Object%20Reference) (OtherActor :type Actor%20Object%20Reference) (OtherComp :type Primitive%20Component%20Object%20Reference) (OtherBodyIndex :type Integer) (bFromSweep :type Boolean) (SweepResult :type Hit%20Result%20Structure%20%28by%20ref%29))
  (Utilities|Casting|CastToSoul_BP OtherActor)
  (Variables|Default|SetTeleportationLocation (Transformation|GetWorldLocation (Variables|Default|GetTargetPoint4))))

(event OnComponentBeginOverlap(TriggerVolume5)
  (params (OverlappedComponent :type Primitive%20Component%20Object%20Reference) (OtherActor :type Actor%20Object%20Reference) (OtherComp :type Primitive%20Component%20Object%20Reference) (OtherBodyIndex :type Integer) (bFromSweep :type Boolean) (SweepResult :type Hit%20Result%20Structure%20%28by%20ref%29))
  (Utilities|Casting|CastToSoul_BP OtherActor)
  (Variables|Default|SetTeleportationLocation (Transformation|GetWorldLocation (Variables|Default|GetTargetPoint5))))

(event Custom|TeleportationAttempt
  (bind (_teleportationlocation_x _teleportationlocation_y _teleportationlocation_z) (|getTeleportationXY))
  (bind _assoul_bp (Utilities|Casting|CastToSoul_BP (stale OnComponentBeginOverlap(TeleportationVolume) OtherActor)))
  (if (not (Utilities|Enum|Equal(Enum) (Variables|/Game/Character/Soul_BP.Soul_BP_C|GetElementalState _assoul_bp) "NewEnumerator1"))
    (Audio|PlaySound2D (Variables|Default|GetSound) 1.0 1.0 0.0 0 0)
    (Transformation|Teleport _assoul_bp (Math|Vector|MakeVector _teleportationlocation_x _teleportationlocation_y _teleportationlocation_z) (|getRotation _assoul_bp))))

(event EventBeginPlay
  (Variables|Default|SetTeleportationLocation (Transformation|GetWorldLocation (Variables|Default|GetDefaultTargetPoint))))

(fn ConstructionScript)