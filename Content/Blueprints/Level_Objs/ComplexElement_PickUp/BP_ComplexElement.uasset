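; Complex element pickup (Magma, Mud or Sand) that the player's Soul can break down into Earth plus a matching simple element.
; BeginPlay uses the type to set the body material and second element (Fire, Water or Air).
; Overlapping the box enables input and shows a hint; pressing E spends an acquired catalyst.
; Breakdown spawns both pickups on opposite sides, perpendicular to the player's direction, plays a sound and destroys itself.
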(event OnComponentBeginOverlap(Box)
  (params (OverlappedComponent :type Primitive%20Component%20Object%20Reference) (OtherActor :type Actor%20Object%20Reference) (OtherComp :type Primitive%20Component%20Object%20Reference) (OtherBodyIndex :type Integer) (bFromSweep :type Boolean) (SweepResult :type Hit%20Result%20Structure%20%28by%20ref%29))
  (bind _assoul_bp (Utilities|Casting|CastToSoul_BP OtherActor))
  (Variables|Default|SetSoulBpRef _assoul_bp)
  (Input|EnableInput (Game|GetPlayerController 0))
  (Default|AddHintMessage (Variables|Default|GetSoulGameStateRef) "Press \"E\" to Break the Complex Element down"))

(event OnComponentEndOverlap(Box)
  (params (OverlappedComponent :type Primitive%20Component%20Object%20Reference) (OtherActor :type Actor%20Object%20Reference) (OtherComp :type Primitive%20Component%20Object%20Reference) (OtherBodyIndex :type Integer))
  (Utilities|Casting|CastToSoul_BP OtherActor)
  (Input|DisableInput (Game|GetPlayerController 0))
  (Default|ClearHintMessage (Variables|Default|GetSoulGameStateRef)))

(event Custom|BreakDownToEarth
  (bind _returnvalue (Transformation|GetActorLocation))
  (bind _soulbpref (Variables|Default|GetSoulBpRef))
  (bind _distancetobreak (Variables|Usage|GetDistanceToBreak))
  (bind (_x _y) (Math|Vector|BreakVector _returnvalue))
  (bind _rootcomponent (Variables|/Script/Engine.Actor|GetRootComponent _soulbpref))
  (bind _returnvalue_2 (Transformation|GetWorldLocation _rootcomponent))
  (bind (_x_2 _y_2) (Math|Vector|BreakVector _returnvalue_2))
  (bind _returnvalue_3 (- (Math|Vector|MakeVector _x _y 0.0) (Math|Vector|MakeVector _x_2 _y_2 0.0)))
  (bind _returnvalue_4 (Class|KismetMathLibrary|VectorNormal2D _returnvalue_3 0.0001))
  (bind _returnvalue_5 (* (.x _returnvalue_4) -1.0))
  (bind _returnvalue_6 (Math|Vector2D|MakeVector2D (.y _returnvalue_4) _returnvalue_5))
  (bind _returnvalue_7 (* _returnvalue_6 _distancetobreak))
  ;[1 1 1] BreakDown
  (Game|SpawnActorfromClass "/Game/Blueprints/Level_Objs/Earth_PickUp/BP_pickableEarth.BP_pickableEarth_C" (Math|Transform|MakeTransform (+ _returnvalue (Math|Conversions|ToVector(Vector2D) _returnvalue_7)) "0, 0, 0" "1,1,1") "Undefined" 0 0)
  (Game|SpawnActorfromClass (Variables|Components|GetSimpleElementToBreakTo) (Math|Transform|MakeTransform (+ _returnvalue (Math|Conversions|ToVector(Vector2D) (* _returnvalue_7 -1.0))) "0, 0, 0" "1,1,1") "Undefined" 0 0)
  (bind _returnvalue_8 (Audio|SpawnSoundatLocation "/Game/Audio/SFX/SFX_ElementBreak.SFX_ElementBreak" (Transformation|GetActorLocation) "0, 0, 0" 1.0 1.0 0.0 0 0))
  (Audio|Components|Audio|Play _returnvalue_8 0.0)
  (Actor|DestroyActor))

(event EventBeginPlay
  (bind _body (Variables|Default|GetBody))
  (bind _assoul_game_state_base (Utilities|Casting|CastToSoulGameStateBase (Game|GetGameState)))
  (Variables|Default|SetSoulGameStateRef _assoul_game_state_base)
  (switch Utilities|FlowControl|Switch|SwitchonComplexElementsEnum (Variables|Usage|GetComplexElementType)
    (:NewEnumerator0
      (Variables|Components|SetSimpleElementToBreakTo "/Game/Blueprints/Level_Objs/Fire_PickUp/BP_pickableFire.BP_pickableFire_C")
      (Rendering|Material|SetMaterial _body 0 "/Game/Blueprints/Level_Objs/ComplexElement_PickUp/M_Complex_Lava.M_Complex_Lava"))
    (:NewEnumerator1
      (Variables|Components|SetSimpleElementToBreakTo "/Game/Blueprints/Level_Objs/Water_PickUp/BP_pickableWater.BP_pickableWater_C")
      (Rendering|Material|SetMaterial _body 0 "/Game/Blueprints/Level_Objs/ComplexElement_PickUp/M_Complex_Mud.M_Complex_Mud"))
    (:NewEnumerator2
      (Variables|Components|SetSimpleElementToBreakTo "/Game/Blueprints/Level_Objs/Air_PickUp/BP_pickableAir.BP_pickableAir_C")
      (Rendering|Material|SetMaterial _body 0 "/Game/Blueprints/Level_Objs/ComplexElement_PickUp/M_Complex_Sand.M_Complex_Sand"))))

(event Collision|EventActorBeginOverlap
  (params (OtherActor :type Actor%20Object%20Reference)))

(event EventTick
  (params (DeltaSeconds :type Float%20%28single-precision%29)))

(event Input|KeyboardEvents|E
  (params (Key :type Key%20Structure :default "None"))
  (bind _soulgamestateref (Variables|Default|GetSoulGameStateRef))
  (:Pressed
    (if (Variables|/Game/Blueprints/SoulGameStateBase.SoulGameStateBase_C|GetIsACatalystAcquired (Variables|Default|GetSoulGameStateRef))
      (Default|CatalystWasted _soulgamestateref)
      (CallFunction|BreakDowntoEarth)
      (else
        (Default|AddHintMessage _soulgamestateref "Need Catalyst to Break it down")))))

(fn ConstructionScript)