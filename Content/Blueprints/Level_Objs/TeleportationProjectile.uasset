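; Looping teleportation projectile for the teleportation puzzle, which sends Soul_BP back to the puzzle's TeleportationLocation on contact.
; A timeline scaled by Duration moves the object along a spline, keeping its starting offset.
; At the path's end or on a hit it explodes with sound and particles, resets to the initial position and relaunches after a delay.
; Souls in one specific elemental state are unaffected by the capsule overlap.
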(event OnComponentBeginOverlap(Capsule)
  (params (OverlappedComponent :type Primitive%20Component%20Object%20Reference) (OtherActor :type Actor%20Object%20Reference) (OtherComp :type Primitive%20Component%20Object%20Reference) (OtherBodyIndex :type Integer) (bFromSweep :type Boolean) (SweepResult :type Hit%20Result%20Structure%20%28by%20ref%29))
  (bind _assoul_bp (Utilities|Casting|CastToSoul_BP OtherActor))
  (if (not (Utilities|Enum|Equal(Enum) (Variables|/Game/Character/Soul_BP.Soul_BP_C|GetElementalState _assoul_bp) "NewEnumerator1"))
    (bind _asteleportation_puzzle (Utilities|Casting|CastToTeleportationPuzzle (Variables|Default|GetTeleportationSystem)))
    (Utilities|FlowControl|Sequence
      (:then_0
        (bind _value (Timeline|SplineTimeline Stop)
          (:Update
            (Transformation|SetWorldLocation (Variables|Default|GetObject) (- (Spline|GetLocationatDistanceAlongSpline (Variables|Default|GetSpline) (Math|Float|Lerp 0.0 (Spline|GetSplineLength (Variables|Default|GetSpline)) _value) "World") (Variables|Default|GetsplineOffsetvec)) false false))
          (:Finished
            (CallFunction|DestroyandRespawn))))
      (:then_1
        (CallFunction|DestroyandRespawn)
        (Transformation|Teleport OtherActor (Variables|/Game/Blueprints/Level_Objs/TeleportationPuzzle.TeleportationPuzzle_C|GetTeleportationLocation _asteleportation_puzzle) (.rotation (Transformation|GetActorTransform)))))))

(event Custom|MoveOverSpline
  (Components|Timeline|SetPlayRate (Variables|Default|GetSplineTimeline) (/ 1.0 (Variables|Usage|GetDuration)))
  (Variables|Default|SetsplineOffsetvec (- (Spline|GetLocationatDistanceAlongSpline (Variables|Default|GetSpline) 0.0 "World") (Transformation|GetWorldLocation (Variables|Default|GetObject))))
  (bind _value (Timeline|SplineTimeline PlayFromStart)
    (:Update
      (Transformation|SetWorldLocation (Variables|Default|GetObject) (- (Spline|GetLocationatDistanceAlongSpline (Variables|Default|GetSpline) (Math|Float|Lerp 0.0 (Spline|GetSplineLength (Variables|Default|GetSpline)) _value) "World") (Variables|Default|GetsplineOffsetvec)) false false))
    (:Finished
      (CallFunction|DestroyandRespawn))))

(event Custom|DestroyAndRespawn
  (bind _object (Variables|Default|GetObject))
  (bind _returnvalue (Transformation|GetWorldLocation _object))
  (Audio|SpawnSoundatLocation "/Game/Audio/SFX/FireOut_SoundCue.FireOut_SoundCue" _returnvalue "0, 0, 0" 1.0 1.0 0.0 0 0)
  (Effects|SpawnEmitteratLocation "/Game/StarterContent/Particles/P_Explosion.P_Explosion" _returnvalue)
  (Transformation|SetWorldLocation (Variables|Default|GetObject) (Variables|Default|GetInitialCoord) false true)
  (Utilities|FlowControl|Delay (Variables|Default|GetDelay))
  (CallFunction|MoveOverSpline))

(event EventBeginPlay
  (Variables|Default|SetInitialCoord (Transformation|GetActorLocation))
  (CallFunction|MoveOverSpline))

(fn ConstructionScript)