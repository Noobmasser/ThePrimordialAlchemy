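; BP_pickableEarth is a level pickup that grants the Earth acquisition when the player soul touches it.
; On BeginPlay it caches the SoulGameStateBase reference.
; A Box overlap with Soul_BP fires the PickUp event, which notifies the game state through EarthAcquired, plays a 2D sound and destroys the actor.
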(event OnComponentBeginOverlap(Box)
  (params (OverlappedComponent :type Primitive%20Component%20Object%20Reference) (OtherActor :type Actor%20Object%20Reference) (OtherComp :type Primitive%20Component%20Object%20Reference) (OtherBodyIndex :type Integer) (bFromSweep :type Boolean) (SweepResult :type Hit%20Result%20Structure%20%28by%20ref%29))
  (Utilities|Casting|CastToSoul_BP OtherActor)
  (CallFunction|PickUp))

(event EventBeginPlay
  (bind _assoul_game_state_base (Utilities|Casting|CastToSoulGameStateBase (Game|GetGameState)))
  (Variables|Default|SetSoulGameState_ref _assoul_game_state_base))

(event Collision|EventActorBeginOverlap
  (params (OtherActor :type Actor%20Object%20Reference)))

(event EventTick
  (params (DeltaSeconds :type Float%20%28single-precision%29)))

(event EventPickUp
  (Default|EarthAcquired (Variables|Default|GetSoulGameState_ref))
  (Audio|SpawnSound2D "/Game/Audio/VFX/Elements/VFX_Earth.VFX_Earth" 1.0 1.0 0.0 0)
  (Actor|DestroyActor))

(fn ConstructionScript)