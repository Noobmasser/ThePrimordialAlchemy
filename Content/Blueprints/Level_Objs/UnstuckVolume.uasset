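; UnstuckVolume is a level volume that rescues the player's Soul_BP character when it gets stuck inside it.
; Box overlap begin and end events toggle a stuck flag for the cached player character.
; Tick accumulates time while the flag is set and resets it otherwise, teleporting the character to the TargetPoint's transform once it has stayed inside for a few seconds.
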(event OnComponentBeginOverlap(Box)
  (params (OverlappedComponent :type Primitive%20Component%20Object%20Reference) (OtherActor :type Actor%20Object%20Reference) (OtherComp :type Primitive%20Component%20Object%20Reference) (OtherBodyIndex :type Integer) (bFromSweep :type Boolean) (SweepResult :type Hit%20Result%20Structure%20%28by%20ref%29))
  (if (== OtherActor (Variables|Default|GetSoulCharacterRef))
    (Variables|Default|SetisStuck true)))

(event OnComponentEndOverlap(Box)
  (params (OverlappedComponent :type Primitive%20Component%20Object%20Reference) (OtherActor :type Actor%20Object%20Reference) (OtherComp :type Primitive%20Component%20Object%20Reference) (OtherBodyIndex :type Integer))
  (if (== OtherActor (Variables|Default|GetSoulCharacterRef))
    (Variables|Default|SetisStuck false)))

(event EventBeginPlay
  (bind _assoul_bp (Utilities|Casting|CastToSoul_BP (Game|GetPlayerCharacter 0)))
  (Variables|Default|SetSoulCharacterRef _assoul_bp))

(event Collision|EventActorBeginOverlap
  (params (OtherActor :type Actor%20Object%20Reference)))

(event EventTick
  (params (DeltaSeconds :type Float%20%28single-precision%29))
  (bind _targetpoint (Variables|Default|GetTargetPoint))
  (bind _returnvalue (Transformation|GetWorldTransform _targetpoint))
  (if (Variables|Default|GetisStuck)
    (Variables|Default|SetTimeStuck (+ (Variables|Default|GetTimeStuck) DeltaSeconds))
    (if (>= (Variables|Default|GetTimeStuck) 3.0)
      (Transformation|Teleport (Variables|Default|GetSoulCharacterRef) (.location _returnvalue) (.rotation _returnvalue)))
    (else
      (Variables|Default|SetTimeStuck 0.0))))

(fn ConstructionScript)