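; A destructible barrier that hides and loses collision when it takes any damage, then respawns after SpawnTime.
; A DoOnce gates destruction until the timer-driven Spawn restores visibility and the collision setting cached at BeginPlay.
; HintBox overlaps with Soul_BP show a Fire-form attack hint through SoulGameStateBase while the wall stands, clearing it on exit or destruction.
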(event OnComponentBeginOverlap(HintBox)
  (params (OverlappedComponent :type Primitive%20Component%20Object%20Reference) (OtherActor :type Actor%20Object%20Reference) (OtherComp :type Primitive%20Component%20Object%20Reference) (OtherBodyIndex :type Integer) (bFromSweep :type Boolean) (SweepResult :type Hit%20Result%20Structure%20%28by%20ref%29))
  (Utilities|Casting|CastToSoul_BP OtherActor)
  (if (not (Variables|Default|GetisDestroyed))
    (Default|AddHintMessage (Variables|Default|GetSoulGameStateRef) "In the Fire form, aim and press LMB to destroy the barrier")))

(event OnComponentEndOverlap(HintBox)
  (params (OverlappedComponent :type Primitive%20Component%20Object%20Reference) (OtherActor :type Actor%20Object%20Reference) (OtherComp :type Primitive%20Component%20Object%20Reference) (OtherBodyIndex :type Integer))
  (Utilities|Casting|CastToSoul_BP OtherActor)
  (Default|ClearHintMessage (Variables|Default|GetSoulGameStateRef)))

(event Custom|Spawn
  (bind _destructablewall (Variables|Default|GetDestructableWall))
  (bind _destructablewall_2 (Variables|Default|GetDestructableWall))
  (Rendering|SetVisibility _destructablewall true false)
  (Collision|SetCollisionEnabled _destructablewall_2 (Variables|LocalVariables|GetCollision%20Enabled))
  (Variables|Default|SetisDestroyed false)
  (Utilities|Time|ClearandInvalidateTimerbyHandle (Variables|LocalVariables|GetSpawnTimer))
  (Utilities|FlowControl|DoOnce false) ; enters at Reset
)

(event Custom|Destroy
  (Utilities|FlowControl|DoOnce false
    (:Completed
      (bind _returnvalue (Utilities|Time|SetTimerbyEvent (delegate Custom|Spawn) (Variables|Usage|GetSpawnTime)))
      (Variables|LocalVariables|SetSpawnTimer _returnvalue)
      (Rendering|SetVisibility (Variables|Default|GetDestructableWall) false false)
      (Collision|SetCollisionEnabled (Variables|Default|GetDestructableWall) "NoCollision")
      (Variables|Default|SetisDestroyed true)
      (Default|ClearHintMessage (Variables|Default|GetSoulGameStateRef)))))

(event EventBeginPlay
  (Variables|LocalVariables|SetCollision%20Enabled (Collision|GetCollisionEnabled (Variables|Default|GetDestructableWall)))
  (bind _assoul_game_state_base (Utilities|Casting|CastToSoulGameStateBase (Game|GetGameState)))
  (Variables|Default|SetSoulGameStateRef _assoul_game_state_base))

(event Game|Damage|EventAnyDamage
  (params (Damage :type Float%20%28single-precision%29) (DamageType :type Damage%20Type%20Object%20Reference) (InstigatedBy :type Controller%20Object%20Reference) (DamageCauser :type Actor%20Object%20Reference))
  (CallFunction|Destroy))

(fn ConstructionScript)