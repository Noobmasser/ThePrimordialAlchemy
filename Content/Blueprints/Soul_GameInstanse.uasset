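; Soul_GameInstanse is a game instance Blueprint that tracks level progression and the Earth count the current level needs.
; StartNextLevel advances an index through a Levels array, copies that entry's NeededEarthCount and opens its level by name.
; After the last level it sets GameHasEnded and wraps back to the first level, clearing the flag on any other advance.
; A getter exposes the current NeededEarthCount.
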(fn GetNeededEarthCount
  (return (Variables|Default|GetNeededEarthCount)))

(fn StartNextLevel
  (if (== (+ (Variables|Default|GetCurrentLevelIndex) 1) (Utilities|Array|Length (Variables|Default|GetLevels)))
    (Variables|Default|SetGameHasEnded true)
    (bind _output_get (Variables|Default|SetCurrentLevelIndex 0))
    (Variables|Default|SetNeededEarthCount (.neededearthcount (Utilities|Array|Get(acopy) (Variables|Default|GetLevels) _output_get)))
    (Game|OpenLevel(byName) (.levelname (Utilities|Array|Get(acopy) (Variables|Default|GetLevels) _output_get)))
    (else
      (Variables|Default|SetGameHasEnded false)
      (bind _output_get_2 (Variables|Default|SetCurrentLevelIndex (+ (Variables|Default|GetCurrentLevelIndex) 1)))
      (Variables|Default|SetNeededEarthCount (.neededearthcount (Utilities|Array|Get(acopy) (Variables|Default|GetLevels) _output_get_2)))
      (Game|OpenLevel(byName) (.levelname (Utilities|Array|Get(acopy) (Variables|Default|GetLevels) _output_get_2))))))